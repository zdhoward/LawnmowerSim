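; Lawn tile floor Blueprint whose grass can be mowed or damaged, with an FMOD sound for each.
; Grass collision is disabled at BeginPlay, and Tick triggers Mowed while State is true.
; Mowed and Damaged both hide the grass and set IsMowed, while Damaged also swaps the tile material to LawnMowed.
; IsMowed and IsDamaged guard against repeats, so a mowed tile can still be damaged.
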(event `self.ReceiveBeginPlay`
  (`PrimitiveComponent.SetCollisionEnabled` (`self.Grass`) "NoCollision"))

(event `self.ReceiveTick`
  (params (DeltaSeconds :type "Float (single-precision)"))
  (if (`self.state`)
    (`self.Event Mowed`)))

(event `Event Damaged`
  (if (not (`self.isDamaged`))
    (`FMODAudioComponent.Play` (`self.FMOD Destroyed`))
    (`PrimitiveComponent.SetMaterial` (`self.StaticMeshComponent`) 0 "/Game/MyGame/Materials/lawnMowed.lawnMowed")
    (set `self.isDamaged` true)
    (`SceneComponent.SetHiddenInGame` (`self.Grass`) true false :!label _label)
    (set `self.isMowed` true)))

(event `Event Mowed`
  (if (not (`self.isMowed`))
    (`FMODAudioComponent.Play` (`self.FMOD Mowed`))
    (goto _label)))

(fn `UserConstructionScript`)