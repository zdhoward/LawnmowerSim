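; Enemy AI character that chases a seen player, attacks on arrival and damages the lawn tiles it walks over.
; Pawn sensing starts an AI move, and reaching the player triggers an FMOD attack sound and a Damage call.
; Each tick traces downward to damage the tile below and checks health, which its Damage event decrements.
; At zero health it plays a death sound, increments the player's kill count and destroys itself.
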(event `self.PawnSensing.OnSeePawn`
  (params (Pawn :type "Pawn Object Reference"))
  (bind _asfull_player_character (cast `/Game/MyGame/Blueprints/Player/FullPlayerCharacter` Pawn))
  (`|AIMoveTo` self (0.0 0.0 0.0) _asfull_player_character
    (:`OnSuccess`
      (`self.Attack`))))

(event `Attack`
  (`FMODAudioComponent.Play` (`self.FMOD Attack`))
  (`/Game/MyGame/Blueprints/Player/FullPlayerCharacter.Damage` (stale `self.PawnSensing.OnSeePawn` _asfull_player_character) 0))

(event `self.ReceiveBeginPlay`
  (`FMODAudioComponent.Play` (`self.FMOD Spawn`))
  (`FMODAudioComponent.Play` (`self.FMOD Warcry`)))

(event `self.ReceiveTick`
  (params (DeltaSeconds :type "Float (single-precision)"))
  (bind _location (.location (`self.GetTransform`)))
  (`|ExecutionSequence`
    (:`then_0`
      ;[1 1 1] RaycastToGround
      (bind _outhit (`KismetSystemLibrary.LineTraceSingleForObjects` _location (+ _location (0.0 0.0 -150.0)) (`|MakeArray` "ObjectTypeQuery1" :!type "EObjectTypeQuery Enum")))
      (bind _aslawn_tile_blueprint (cast `/Game/MyGame/Blueprints/Floor/LawnTile_Blueprint` (`.HitActor` (`GameplayStatics.BreakHitResult` _outhit))))
      (`/Game/MyGame/Blueprints/Floor/LawnTile_Blueprint.Event Damaged` _aslawn_tile_blueprint))
    (:`then_1`
      ;[1 1 1] Die
      (if (<= (`self.Health`) 0)
        (`FMODAudioComponent.Play` (`self.FMOD Die`))
        (bind _asfull_player_character (cast `/Game/MyGame/Blueprints/Player/FullPlayerCharacter` (`GameplayStatics.GetPlayerCharacter` 0)))
        (bind _result (`/Engine/EditorBlueprintResources/StandardMacros.IncrementInt` (`/Game/MyGame/Blueprints/Player/FullPlayerCharacter.Kills` _asfull_player_character))
          (:`  `
            (set `/Game/MyGame/Blueprints/Player/FullPlayerCharacter.Kills` _result _asfull_player_character)
            (`self.K2_DestroyActor`)))))))

(event `Damage`
  ;[1 1 1] Take Damage
  (bind _result (`/Engine/EditorBlueprintResources/StandardMacros.DecrementInt` (`self.Health`))
    (:`  `
      (set `self.Health` _result))))

(fn `UserConstructionScript`)