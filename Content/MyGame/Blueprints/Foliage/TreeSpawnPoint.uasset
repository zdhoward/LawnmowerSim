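; Tree spawn point Blueprint that displays a randomly chosen tree when play begins.
; On BeginPlay it sets the Tree component to a random mesh from the Trees array, then gives it a random height offset, yaw and independent per-axis scale.
; The variation is rolled at runtime, as the construction script is empty.
; An unconnected AddInstanceWorldSpace node never runs.
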(event `self.ReceiveBeginPlay`
  (bind _trees (`self.Trees`))
  (bind _tree (`self.tree`))
  (bind _returnvalue (`KismetMathLibrary.Conv_IntToDouble` (+ (`KismetMathLibrary.RandomInteger` 5) 13)))
  (`StaticMeshComponent.SetStaticMesh` _tree (`|GetArrayItem` _trees (`KismetMathLibrary.RandomInteger` (`KismetArrayLibrary.Array_Length` _trees))))
  (`SceneComponent.K2_SetRelativeTransform` _tree (`KismetMathLibrary.MakeTransform` (`KismetMathLibrary.MakeVector` 0.0 0.0 (`KismetMathLibrary.Conv_IntToDouble` (+ (`KismetMathLibrary.RandomInteger` 10) 120))) (`KismetMathLibrary.MakeRotator` 0.0 0.0 (`KismetMathLibrary.Conv_IntToDouble` (`KismetMathLibrary.RandomInteger` 360))) (`KismetMathLibrary.MakeVector` _returnvalue _returnvalue _returnvalue)) false false))

(fn `UserConstructionScript`)