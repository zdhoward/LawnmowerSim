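; Time-of-day sky sphere that drives a day/night cycle by rotating its directional light.
; BeginPlay derives an hour's length from DayLengthInMinutes, and Tick advances Hour while not paused, resetting it at 24.
; Hour maps linearly to sun pitch, with yaw taken from the sphere, then UpdateSunDirection refreshes the sky.
; The construction script calls its parent and applies the same rotation, so the starting hour shows in the editor.
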(event `self.ReceiveBeginPlay`
  ;[1 1 1] Set Time Context
  (bind _output_get (set `self.OneDay` (* (`self.DayLengthInMinutes`) 60.0)))
  (set `self.OneHour` (/ _output_get 24.0)))

(event `self.ReceiveTick`
  (params (DeltaSeconds :type "Float (single-precision)"))
  (bind (_returnvalue_roll _returnvalue_pitch _returnvalue_yaw) (`KismetMathLibrary.BreakRotator` (`self.K2_GetActorRotation`)))
  (bind _hour (`self.Hour`))
  (bind _directional_light_actor (`self.Directional light actor`))
  (bind _returnvalue (+ (/ DeltaSeconds (`self.OneHour`)) _hour))
  ;[1 1 1] Make Sun Rise and Set
  (if (not (`self.isPaused`))
    (if (>= _returnvalue 24.0)
      (set `self.Hour` 0.0)
      (else
        (set `self.Hour` _returnvalue)))
    (bind _output_get (set `self.SunAngle` (+ (* (/ _hour 6.0) 90.0) 90.0)))
    (`/Engine/EditorBlueprintResources/StandardMacros.IsValid` _directional_light_actor
      (:`Is Valid`
        (`self.K2_SetActorRotation` _directional_light_actor (`KismetMathLibrary.MakeRotator` 0.0 _output_get _returnvalue_yaw) false)
        (`self.UpdateSunDirection`)))))

(fn `UserConstructionScript`
  (bind (_returnvalue_roll _returnvalue_pitch _returnvalue_yaw) (`KismetMathLibrary.BreakRotator` (`self.K2_GetActorRotation`)))
  (bind _directional_light_actor (`self.Directional light actor`))
  (`parent.UserConstructionScript`)
  (bind _output_get (set `self.SunAngle` (+ (* (/ (`self.Hour`) 6.0) 90.0) 90.0)))
  (`/Engine/EditorBlueprintResources/StandardMacros.IsValid` _directional_light_actor
    (:`Is Valid`
      (`self.K2_SetActorRotation` _directional_light_actor (`KismetMathLibrary.MakeRotator` 0.0 _output_get _returnvalue_yaw) false)
      (`self.UpdateSunDirection`))))